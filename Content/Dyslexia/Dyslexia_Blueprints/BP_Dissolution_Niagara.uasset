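; BP_Dissolution_Niagara is an actor that replaces a target actor with a Niagara dissolve effect.
; Two seconds after BeginPlay it calls Dissolve on its Actor variable, then hides that actor in game.
; Dissolve feeds the target's StaticMeshComponent and first material into the Niagara system's user variables, enables auto-destroy and resets the system to play the effect.
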(event Custom|Dissolve
  (params (Actor :type Actor%20Object%20Reference))
  (bind _niagara (Variables|Default|GetNiagara))
  (bind _niagara_2 (Variables|Default|GetNiagara))
  (Variables|Default|SetActor Actor)
  (Utilities|IsValid (Actor|GetComponentbyClass (Variables|Default|GetActor) "/Script/Engine.StaticMeshComponent")
    (:Is%20Valid
      (Class|NiagaraFunctionLibrary|OverrideSystemUserVariableStaticMeshComponent _niagara "StaticMesh" (Actor|GetComponentbyClass (Variables|Default|GetActor) "/Script/Engine.StaticMeshComponent"))
      (Class|NiagaraComponent|SetVariableMaterial _niagara "Material" (Rendering|Material|GetMaterial (Actor|GetComponentbyClass (Variables|Default|GetActor) "/Script/Engine.StaticMeshComponent") 0))
      (Class|NiagaraComponent|SetAutoDestroy _niagara_2 true)
      (Components|Activation|SetAutoActivate _niagara_2 false)
      (Niagara|ResetSystem _niagara_2))))

(event EventBeginPlay
  (Utilities|FlowControl|Delay 2.0)
  (CallFunction|Dissolve (Variables|Default|GetActor))
  (Rendering|SetActorHiddenInGame (Variables|Default|GetActor) true))

(event Collision|EventActorBeginOverlap
  (params (OtherActor :type Actor%20Object%20Reference)))

(event EventTick
  (params (DeltaSeconds :type Float%20%28single-precision%29)))

(fn ConstructionScript)